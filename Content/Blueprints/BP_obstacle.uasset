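; BP_obstacle is a frog obstacle that moves between a road's left and right spawn points and ragdolls when struck by a vehicle.
; Tick calls MoveFrog, which casts the root component's owner to RoadOutline, then alternates VInterpTo moves through looping Gates.
; FrogBubble overlap with a VehicleBlueprint calls its HitFrog and enables mesh physics, while a direct mesh hit only enables physics.
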(event `self.ReceiveTick`
  (params (DeltaSeconds :type "Float (single-precision)"))
  (`self.MoveFrog`))

(event `self.SkeletalMesh.OnComponentHit`
  (params (HitComponent :type "PrimitiveComponent Object Reference") (OtherActor :type "Actor Object Reference") (OtherComp :type "PrimitiveComponent Object Reference") (NormalImpulse :type "Vector Structure") (Hit :type "HitResult Structure (by ref)"))
  ;[1 1 1] Collision event for frog object.
  (bind _asvehicle_blueprint (cast `/Game/VehicleAdvBP/Blueprints/VehicleBlueprint` OtherActor))
  (`PrimitiveComponent.SetSimulatePhysics` (`self.SkeletalMesh`) true))

(event `self.FrogBubble.OnComponentBeginOverlap`
  (params (OverlappedComponent :type "PrimitiveComponent Object Reference") (OtherActor :type "Actor Object Reference") (OtherComp :type "PrimitiveComponent Object Reference") (OtherBodyIndex :type Integer) (bFromSweep :type Boolean) (SweepResult :type "HitResult Structure (by ref)"))
  ;[1 1 1] Collision event for custom bubble put around frog object. Makes frog object ragdoll.
  (bind _asvehicle_blueprint (cast `/Game/VehicleAdvBP/Blueprints/VehicleBlueprint` OtherActor))
  (`/Game/VehicleAdvBP/Blueprints/VehicleBlueprint.HitFrog` _asvehicle_blueprint)
  (`PrimitiveComponent.SetSimulatePhysics` (`self.SkeletalMesh`) true))

(fn `MoveFrog`
  (bind _skeletalmesh (`self.SkeletalMesh`))
  (bind _skeletalmesh_2 (`self.SkeletalMesh`))
  (bind _returnvalue (`SceneComponent.K2_GetComponentLocation` _skeletalmesh))
  (bind _returnvalue_2 (`SceneComponent.K2_GetComponentLocation` _skeletalmesh_2))
  (bind _asroad_outline (cast `/Game/Blueprints/RoadOutline` (`ActorComponent.GetOwner` (`self.DefaultSceneRoot`))))
  (bind _output_get (set `self.RoadReference` _asroad_outline))
  (`|ExecutionSequence`
    (:`then_0`
      (bind _returnvalue_3 (`SceneComponent.K2_GetComponentLocation` (`/Game/Blueprints/RoadOutline.SpawnPointL` _output_get)))
      (`SceneComponent.K2_SetWorldLocation` _skeletalmesh (`KismetMathLibrary.VInterpTo` _returnvalue _returnvalue_3) false false :!label _label)
      (`|ExecutionSequence`
        (:`then_0`
          (`/Engine/EditorBlueprintResources/StandardMacros.Gate` true :!label _label_2
            (:`Exit`
              (goto _label))))
        (:`then_1`
          (if (== _returnvalue _returnvalue_3 :`ErrorTolerance` 10.0)
            (`|ExecutionSequence`
              (:`then_0`
                (goto _label_2 :!via `Close`))
              (:`then_1`
                (`|ExecutionSequence`
                  (:`then_0`
                    (bind _returnvalue_4 (`SceneComponent.K2_GetComponentLocation` (`/Game/Blueprints/RoadOutline.SpawnPointR` _output_get)))
                    (`SceneComponent.K2_SetWorldLocation` _skeletalmesh_2 (`KismetMathLibrary.VInterpTo` _returnvalue_2 _returnvalue_4 0.0 2.0) false false :!label _label_3)
                    (`|ExecutionSequence`
                      (:`then_0`
                        (`/Engine/EditorBlueprintResources/StandardMacros.Gate` true :!label _label_4
                          (:`Exit`
                            (goto _label_3))))
                      (:`then_1`
                        (if (== _returnvalue_2 _returnvalue_4 :`ErrorTolerance` 10.0)
                          (`|ExecutionSequence`
                            (:`then_0`
                              (goto _label_4 :!via `Close`))
                            (:`then_1`
                              (goto _label))
                            (:`then_2`
                              (goto _label_2 :!via `Open`)))))))
                  (:`then_1`
                    (goto _label_4 :!via `Open`)))))))))
    (:`then_1`
      (goto _label_2 :!via `Open`))))

(fn `UserConstructionScript`)