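; Road tile actor for an endlessly extending vehicle course, built from pieces that spawn and remove themselves.
; Construction gathers three spawn point transforms and adds a blocker child actor at a random one.
; When the vehicle overlaps EndTrigger, it asks VehicleAdvGameMode to add a floor tile, then destroys itself two seconds later.
; GetAttachTransform exposes the world transform of AttachPoint.
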(event `self.EndTrigger.OnComponentBeginOverlap`
  (params (OverlappedComponent :type "PrimitiveComponent Object Reference") (OtherActor :type "Actor Object Reference") (OtherComp :type "PrimitiveComponent Object Reference") (OtherBodyIndex :type Integer) (bFromSweep :type Boolean) (SweepResult :type "HitResult Structure (by ref)"))
  (cast `/Game/VehicleAdvBP/Blueprints/VehicleBlueprint` OtherActor)
  (bind _asvehicle_adv_game_mode (cast `/Game/VehicleAdvBP/Blueprints/VehicleAdvGameMode` (`GameplayStatics.GetGameMode`)))
  (`/Game/VehicleAdvBP/Blueprints/VehicleAdvGameMode.AddFloorTile` _asvehicle_adv_game_mode)
  (`KismetSystemLibrary.Delay` 2.0)
  (`self.K2_DestroyActor`))

(fn `GetAttachTransform`
  (returns (AttachTransform :type "Transform Structure"))
  ;[1 1 1] Find out where Arrow is in World.
  (return (`SceneComponent.K2_GetComponentToWorld` (`self.AttachPoint`))))

(fn `SetSpawnPoints`
  (set `self.SpawnPoints` (`|MakeArray` (`SceneComponent.GetRelativeTransform` (`self.SpawnPoint`)) (`SceneComponent.GetRelativeTransform` (`self.SpawnPointL`)) (`SceneComponent.GetRelativeTransform` (`self.SpawnPointR`)))))

(fn `SpawnBlocker`
  (bind _spawnpoints (`self.SpawnPoints`))
  (`AddComponent|NODE_AddChildActorComponent-0` :`RelativeTransform` (`|GetArrayItem` _spawnpoints (`KismetMathLibrary.RandomIntegerInRange` 0 (`KismetArrayLibrary.Array_LastIndex` _spawnpoints)))))

(fn `UserConstructionScript`
  (`self.SetSpawnPoints`)
  (`self.SpawnBlocker`))