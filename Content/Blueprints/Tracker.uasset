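; Tracker is a developer-editable settings object that configures the game for a map when play begins.
; On BeginPlay it casts player controller 0 to MyPlayerController, then copies in the save slot, map name, lives, default bests and time limit.
; It then calls StartGameSetup on the controller, followed by its own StartSequence event, which is empty here.
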(event `self.ReceiveBeginPlay`
  ;[1 1 1] Event Begin Play - Get Controller Reference
  (bind _asmy_player_controller (cast `/Game/Blueprints/MyPlayerController` (`GameplayStatics.GetPlayerController` 0)))
  (set `self.ControllerReference` _asmy_player_controller)
  (`self.ApplySettings`)
  (`self.StartSequence`))

(event `ApplySettings`
  (bind _controllerreference (`self.ControllerReference`))
  ;[1 1 1] Apply User Settings When Game Starts. These can be edited from the Tracker object by developers.
  (set `/Game/Blueprints/MyPlayerController.SaveSlot` (`self.SaveGameName`) _controllerreference)
  (set `/Game/Blueprints/MyPlayerController.NameOfMap` (`self.NameOfMap`) _controllerreference)
  (set `/Game/Blueprints/MyPlayerController.MaxLives` (`self.Lives`) _controllerreference)
  (`self.UpdateTimes`)
  (`/Game/Blueprints/MyPlayerController.StartGameSetup` _controllerreference))

(event `StartSequence`)

(fn `UpdateTimes`
  (bind _controllerreference (`self.ControllerReference`))
  ;[1 1 1] Pass values from Tracker to Controller.
  (set `/Game/Blueprints/MyPlayerController.DefaultBestGameTime` (`self.DefaultBestGameTime`) _controllerreference)
  (set `/Game/Blueprints/MyPlayerController.DefaultBestScoreValue` (`self.DefaultBestScore`) _controllerreference)
  (set `/Game/Blueprints/MyPlayerController.MaxGameTime` (`self.MaxGameTime`) _controllerreference))

(fn `UserConstructionScript`)